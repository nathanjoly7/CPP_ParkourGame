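; BP_WallOfDeath is a moving hazard that destroys the third-person player character on overlap and plays a 2D sound.
; From BeginPlay, two timelines loop it along world Y, one adding to its position and the other, played in reverse, subtracting.
; A variable delay separates the outward and return moves, and a short fixed delay precedes each restart.
; Timeline values are per-update increments, so travel distance depends on frame rate.
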(event EventBeginPlay
  (bind _returnvalue (Transformation|GetActorLocation))
  (bind _returnvalue_2 (Transformation|GetActorLocation))
  (bind _newtrack_1 (Timeline|Timeline PlayFromStart)
    (:Update
      (Transformation|SetActorLocation (Math|Vector|MakeVector (.x _returnvalue_2) (+ (.y _returnvalue_2) _newtrack_1) (.z _returnvalue_2)) false false))
    (:Finished
      (Utilities|FlowControl|Delay (Variables|Default|Getdelay))
      (bind _newtrack_1_2 (Timeline|Timeline_0 ReverseFromEnd)
        (:Update
          (Transformation|SetActorLocation (Math|Vector|MakeVector (.x _returnvalue) (- (.y _returnvalue) _newtrack_1_2) (.z _returnvalue)) false false))
        (:Finished
          (Utilities|FlowControl|Delay 0.2)
          (Timeline|Timeline PlayFromStart))))))

(event Collision|EventActorBeginOverlap
  (params (OtherActor :type Actor%20Object%20Reference))
  (bind _asbp_third_person_character (Utilities|Casting|CastToBP_ThirdPersonCharacter OtherActor))
  (Actor|DestroyActor _asbp_third_person_character)
  (Audio|PlaySound2D "/Engine/EditorSounds/Notifications/CompileFailed.CompileFailed" 1.0 1.0 0.0 0 0))

(fn ConstructionScript)