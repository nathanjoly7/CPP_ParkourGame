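; GM_collecte is a game mode Blueprint for a collection game that shows a score widget, tracks score and respawns the player.
; BeginPlay binds OnDeath to the character's destruction, which spawns a replacement at SpawnTransform after a short delay, possesses it and rebinds through RespawnPlayer.
; AddScore accumulates points, and TimeOut pauses the game.
; A leftover chain that destroys the character is unconnected.
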(event Custom|TimeOut
  (Game|SetGamePaused true))

(event Custom|RespawnPlayer
  (bind _asbp_third_person_character (Utilities|Casting|CastToBP_ThirdPersonCharacter (Game|GetPlayerCharacter 0)))
  (Game|BindEventtoOnDestroyed _asbp_third_person_character (delegate Custom|OnDeath)))

(event Custom|OnDeath
  (params (DestroyedActor :type Actor%20Object%20Reference))
  (Utilities|FlowControl|Delay 0.2)
  (bind _returnvalue (Game|SpawnActorfromClass "/Game/ThirdPerson/Blueprints/BP_ThirdPersonCharacter.BP_ThirdPersonCharacter_C" (Variables|Default|GetSpawnTransform) "AdjustIfPossibleButAlwaysSpawn" "MultiplyWithRoot" 0 0))
  (Pawn|Possess (Game|GetPlayerController 0) _returnvalue)
  (CallFunction|RespawnPlayer))

(event EventBeginPlay
  (Utilities|FlowControl|Sequence
    (:then_0
      (bind _returnvalue (UserInterface|CreateWidget "/Game/UI/WB_Score.WB_Score_C"))
      (UserInterface|Viewport|AddtoViewport _returnvalue 0))
    (:then_1
      (bind _asbp_third_person_character (Utilities|Casting|CastToBP_ThirdPersonCharacter (Game|GetPlayerCharacter 0)))
      (Game|BindEventtoOnDestroyed _asbp_third_person_character (delegate Custom|OnDeath)))))

(fn ConstructionScript)

(fn AddScore
  (params (value :type Integer))
  (Variables|Default|Setscore (+ value (Variables|Default|Getscore))))